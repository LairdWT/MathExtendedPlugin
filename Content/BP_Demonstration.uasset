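; Demonstration actor that wanders between four stored locations using a Perlin smooth-step interpolation.
; Tick accumulates time, resets it after roughly two to three seconds and randomly picks a new location enum value.
; That enum selects the target and per-axis delays and durations for LerpToLocation, which moves the actor from its current position via VectorPerlinSmoothStep.
; Other interpolation, falloff and quaternion math nodes sit unused in the graph.
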(event `self.ReceiveTick`
  (params (DeltaSeconds :type "Float (single-precision)"))
  (set `self.Time` (+ DeltaSeconds (`self.Time`)))
  (if (> (`self.Time`) (`KismetMathLibrary.RandomFloatInRange` 2.0 3.0))
    (set `self.Time` 0.0)
    (`self.RandomizeEnumerator`))
  (switch `/MathExtended/ELocations` (`self.ELocationsSet`)
    (:`NewEnumerator0`
      (`self.LerpToLocation` (`self.Time`) (1.0 0.0 0.0) (3.0 6.0 9.0) (`self.K2_GetActorLocation`) (`|GetArrayItem` (`self.Locations`))))
    (:`NewEnumerator1`
      (`self.LerpToLocation` (`self.Time`) (0.0 1.0 0.0) (6.0 9.0 3.0) (`self.K2_GetActorLocation`) (`|GetArrayItem` (`self.Locations`) 1)))
    (:`NewEnumerator2`
      (`self.LerpToLocation` (`self.Time`) (0.0 1.0 0.0) (9.0 3.0 3.0) (`self.K2_GetActorLocation`) (`|GetArrayItem` (`self.Locations`) 2)))
    (:`NewEnumerator3`
      (`self.LerpToLocation` (`self.Time`) (0.0 0.0 0.0) (3.0 3.0 1.0) (`self.K2_GetActorLocation`) (`|GetArrayItem` (`self.Locations`) 3)))))

(event `RandomizeEnumerator`
  ;[1 1 1] Randomize the Selected location Enum
  (set `self.ELocationsSet` (cast `/MathExtended/ELocations` (`KismetMathLibrary.Conv_IntToByte` (`KismetMathLibrary.RandomIntegerInRange` 0 3)))))

(fn `LerpToLocation`
  (params (Time :type "Float (double-precision)") (`Start Delay` :type "Vector Structure") (Duration :type "Vector Structure") (StartLocation :type "Vector Structure") (EndLocation :type "Vector Structure"))
  (`self.K2_SetActorLocation` (`MathExtendedBPLibrary.VectorPerlinSmoothStep` Time `Start Delay` Duration StartLocation EndLocation)))

(fn `UserConstructionScript`)